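; Shift block that triggers a perspective shift on BP_Scientist, alternating between right and the opposite direction.
; A Cube hit with a near straight-up normal passes ShiftRight to the scientist, then flips it and plays a sound.
; UpdateDirection, run at construction and after each flip, mirrors the texture through a dynamic material instance to show the next direction.
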(event `self.Cube.OnComponentHit`
  (params (HitComponent :type "PrimitiveComponent Object Reference") (OtherActor :type "Actor Object Reference") (OtherComp :type "PrimitiveComponent Object Reference") (NormalImpulse :type "Vector Structure") (Hit :type "HitResult Structure (by ref)"))
  (bind _shiftright (`self.ShiftRight`))
  (if (> (`KismetMathLibrary.Dot_VectorVector` (`.Normal` (`GameplayStatics.BreakHitResult` Hit)) (0.0 0.0 1.0)) 0.9)
    (bind _asbp_scientist (cast `/Game/TheMadScientist/Core/BP_Scientist` OtherActor))
    (`/Game/TheMadScientist/Core/BP_Scientist.TriggerPerspectiveShifting` _asbp_scientist _shiftright)
    (set `self.ShiftRight` (not _shiftright))
    (`self.UpdateDirection`)
    (`GameplayStatics.SpawnSound2D` "/Game/TheMadScientist/Ressources/Audio/A_Shift.A_Shift" 1.0 1.0 0.0 null)))

(fn `UpdateDirection`
  (bind _returnvalue (`PrimitiveComponent.CreateDynamicMaterialInstance` (`self.Cube`) 0 null "None"))
  (`MaterialInstanceDynamic.SetScalarParameterValue` _returnvalue "MirrorTexture" (`KismetMathLibrary.Conv_BoolToDouble` (`self.ShiftRight`)))
  (return))

(fn `UserConstructionScript`
  (`parent.UserConstructionScript`)
  (`self.UpdateDirection`))