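; BP_Block_Crate is a destructible crate block that loses one health point each time its TakeDamage event fires.
; At zero health or below, it spawns a Niagara explosion at its location and destroys itself.
; Otherwise, once health falls to the crack threshold, a DoOnce gate swaps its texture to the cracked crate a single time.
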(event `/Game/TheMadScientist/Core/BPI_Damageable.TakeDamage`
  ;[0 0 0] MANAGE TAKE DAMAGE
  (bind _result (`/Engine/EditorBlueprintResources/StandardMacros.DecrementInt` (`self.HealthPoints`))
    (:`  `
      (if (<= _result 0)
        (`NiagaraFunctionLibrary.SpawnSystemAtLocation` "/Game/TheMadScientist/Core/NS_Explosion.NS_Explosion" (`self.K2_GetActorLocation`))
        (`self.K2_DestroyActor`)
        (elif (<= _result (`self.CrackThreshold`))
          (`/Engine/EditorBlueprintResources/StandardMacros.DoOnce` false
            (:`Completed`
              (`self.UpdateTexture` "/Game/TheMadScientist/Ressources/Art/Interactables/Crate/T_Crate_Cracked.T_Crate_Cracked"))))))))

(fn `UserConstructionScript`
  (`parent.UserConstructionScript`))